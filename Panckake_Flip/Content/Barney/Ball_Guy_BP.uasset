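; Player-controlled Blueprint with debug-style key bindings for triggering spawners and moving its capsule.
; Z and X find the weight and ball spawner actors by class and fire their spawn events, while Space prints a message on press and release.
; Right_IA moves the capsule upward in timed steps, looping while its action value is true and feeding world location into a relative-location target.
; Left_IA is empty.
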(event `Key|SpaceBar`
  (params (Key :type "Key Structure"))
  (:`Pressed`
    (`KismetSystemLibrary.PrintString` "Hello" :!label _label))
  (:`Released`
    (goto _label)))

(event `Key|Z`
  (params (Key :type "Key Structure"))
  (:`Pressed`
    (bind _returnvalue (`GameplayStatics.GetActorOfClass` "/Game/Jude/BP_Spawn_Weigt.BP_Spawn_Weigt_C"))
    (`/Game/Jude/BP_Spawn_Weigt.Event Spawner Weight` _returnvalue)))

(event `Key|X`
  (params (Key :type "Key Structure"))
  (:`Pressed`
    (bind _returnvalue (`GameplayStatics.GetActorOfClass` "/Game/Jude/BP_Spawn_Ball.BP_Spawn_Ball_C"))
    (`/Game/Jude/BP_Spawn_Ball.EVent Spawner Ball` _returnvalue)))

(event `EnhancedInput|/Game/Barney/Right_IA`
  (params (ActionValue :type Boolean) (ElapsedSeconds :type "Float (double-precision)") (TriggeredSeconds :type "Float (double-precision)") (InputAction :type "InputAction Object Reference" :default "/Game/Barney/Right_IA.Right_IA"))
  (:`Triggered`
    (if ActionValue :!label _label_2
      (`KismetSystemLibrary.MoveComponentTo` (`self.CapsuleComponent`) (+ (`SceneComponent.K2_GetComponentLocation` (`self.CapsuleComponent`)) (0.0 0.0 50.0)) (struct) false false 0.5)
      (goto _label_2))))

(event `EnhancedInput|/Game/Barney/Left_IA`
  (params (ActionValue :type Boolean) (ElapsedSeconds :type "Float (double-precision)") (TriggeredSeconds :type "Float (double-precision)") (InputAction :type "InputAction Object Reference" :default "/Game/Barney/Left_IA.Left_IA")))

(fn `UserConstructionScript`)