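; BP_Cannon is a cannon that launches BP_Ball on a Spacebar press.
; The Cannon_Switch event enables player input on it.
; When the ball's SeesawBool is false, Spacebar turns on the ball's physics and eases the Cube component quickly forward along X like a piston.
; Unconnected leftover logic covers swapping the seesaw for a cannon, a Timeline-driven power value and weight spawning, none of which runs.
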(event `Cannon_Switch`
  (`self.EnableInput` (`GameplayStatics.GetPlayerController` 0)))

(event `self.ReceiveBeginPlay`)

(event `EnhancedInput|/Game/Barney/Accessiblity/IA_Spacebar`
  (params (ActionValue :type Boolean) (ElapsedSeconds :type "Float (double-precision)") (TriggeredSeconds :type "Float (double-precision)") (InputAction :type "InputAction Object Reference" :default "/Game/Barney/Accessiblity/IA_Spacebar.IA_Spacebar"))
  (:`Triggered`
    (bind _returnvalue (`GameplayStatics.GetActorOfClass` "/Game/Barney/BP_Ball.BP_Ball_C"))
    (if (not (`/Game/Barney/BP_Ball.Seesaw_bool` _returnvalue))
      (bind _returnvalue_2 (`GameplayStatics.GetActorOfClass` "/Game/Barney/BP_Ball.BP_Ball_C"))
      (`PrimitiveComponent.SetSimulatePhysics` (`/Game/Barney/BP_Ball.Sphere` _returnvalue_2) true)
      (`KismetSystemLibrary.MoveComponentTo` (`self.Cube`) (+ (`SceneComponent.RelativeLocation` (`self.Cube`)) (190.0 0.0 0.0)) (struct) false true 0.1))))

(fn `UserConstructionScript`)