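; BP_MovingWall is a wall actor that slides back and forth continuously from BeginPlay.
; Two chained latent MoveComponentTo calls ease the Cube to the WallMovement X/Y/Z relative location, then to its negation, with a fixed duration per leg.
; The custom Loop event calls itself after the second move, so the oscillation around the relative origin repeats indefinitely without Tick or a Timeline.
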(event `Loop`
  (bind _wall_movement_y (`self.Wall Movement Y`))
  (bind _wall_movement_x (`self.Wall Movement X`))
  (bind _cube (`self.Cube`))
  (bind _wall_movement_z (`self.Wall Movement Z`))
  (`KismetSystemLibrary.MoveComponentTo` _cube (`KismetMathLibrary.MakeVector` _wall_movement_x _wall_movement_y _wall_movement_z) (struct) true true 3.5 :!label _label)
  (`KismetSystemLibrary.MoveComponentTo` _cube (`KismetMathLibrary.MakeVector` (/ _wall_movement_x -1) (/ _wall_movement_y -1) (/ _wall_movement_z -1)) (struct) true true 3.5)
  (`self.Loop`))

(event `self.ReceiveBeginPlay`
  (goto _label))

(fn `UserConstructionScript`)