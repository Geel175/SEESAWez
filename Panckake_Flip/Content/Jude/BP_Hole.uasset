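; BP_Hole is the golf hole that ends play when a BP_Ball enters its trigger box while the On flag is set.
; The overlap rates the ball's shot count from Hole In One to Above Par, storing each rating in its own variable.
; It then clears all widgets, shows a new BP_Victory screen and enables the mouse cursor.
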(event `self.Box.OnComponentBeginOverlap`
  (params (OverlappedComponent :type "PrimitiveComponent Object Reference") (OtherActor :type "Actor Object Reference") (OtherComp :type "PrimitiveComponent Object Reference") (OtherBodyIndex :type Integer) (bFromSweep :type Boolean) (SweepResult :type "HitResult Structure (by ref)"))
  (if (`self.On?`)
    (bind _asbp_ball (cast `/Game/Barney/BP_Ball` OtherActor))
    (bind _shots (`/Game/Barney/BP_Ball.Shots` _asbp_ball))
    (if (<= _shots 1)
      (set `self.Hole In one` "Hole In One")
      (elif (<= _shots 2)
        (set `self.Eagle` "Eagle")
        (elif (<= _shots 3)
          (set `self.Birdie` "Birdie")
          (elif (<= _shots 4)
            (set `self.Par` "Par")
            (else
              (set `self.Above Par` "Above Par"))))))
    (`WidgetLayoutLibrary.RemoveAllWidgets`)
    (bind _returnvalue (`|CreateWidget` "/Game/Jude/Widgets/BP_Victory.BP_Victory_C"))
    (`UserWidget.AddToViewport` _returnvalue 0)
    (set `PlayerController.bShowMouseCursor` true (`GameplayStatics.GetPlayerController` 0))))

(fn `UserConstructionScript`)